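; Kickable ball placeholder that turns into a launched ball when the player's foot hits it.
; On the first overlap with BP_Player's FootBox, it plays a kick sound and increments the game instance's KickCounter.
; The player's KickST picks a low, mid or high spawn function, which spawns BP_Ball1, 2 or 3 along the player's rotation with randomized upward pitch.
; The original mesh is then hidden and the actor destroys itself after a delay.
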(event `self.Sphere.OnComponentBeginOverlap`
  (params (OverlappedComponent :type "PrimitiveComponent Object Reference") (OtherActor :type "Actor Object Reference") (OtherComp :type "PrimitiveComponent Object Reference") (OtherBodyIndex :type Integer) (bFromSweep :type Boolean) (SweepResult :type "HitResult Structure (by ref)"))
  (bind _asbp_player (cast `/Game/Player/BP_Player` OtherActor))
  (bind _asbox_collision (cast `BoxComponent` OtherComp))
  (if (== _asbox_collision (`/Game/Player/BP_Player.FootBox` _asbp_player))
    (`/Engine/EditorBlueprintResources/StandardMacros.DoOnce` false
      (:`Completed`
        (`GameplayStatics.PlaySound2D` "/Game/Sound/Kick_QUE.Kick_QUE" 1.0 1.0 0.0 null null)
        (bind _asstruc_kout_game_instance (cast `/Game/Map/StrucKOutGameInstance` (`GameplayStatics.GetGameInstance`)))
        (`/Engine/EditorBlueprintResources/StandardMacros.IncrementInt` (`/Game/Map/StrucKOutGameInstance.KickCounter` _asstruc_kout_game_instance)
          (:`  `
            (switch `int` (`/Game/Player/BP_Player.kickST` _asbp_player)
              (:`1`
                (`self.ball spawn_Low_Func` 10.0 15.0))
              (:`2`
                (`self.ball spawn_Mid_Func` 10.0 20.0))
              (:`3`
                (`self.ball spawn_HI_Func` 10.0 15.0)))
            (`KismetSystemLibrary.Delay` 3.0)
            (`self.K2_DestroyActor`)))))))

(fn `ball spawn_HI_Func`
  (params (min :type "Float (double-precision)") (max :type "Float (double-precision)"))
  (bind _asbp_player (cast `/Game/Player/BP_Player` (`GameplayStatics.GetPlayerPawn` 0)))
  (bind (_returnvalue_roll _returnvalue_pitch _returnvalue_yaw) (`KismetMathLibrary.BreakRotator` (`self.K2_GetActorRotation` _asbp_player)))
  (`|SpawnActorFromClass` "/Game/Map/Ball/BP_Ball3.BP_Ball3_C" (`KismetMathLibrary.MakeTransform` (`SceneComponent.K2_GetComponentLocation` (`self.Ball`)) (`KismetMathLibrary.MakeRotator` _returnvalue_roll (+ _returnvalue_pitch (`KismetMathLibrary.RandomFloatInRange` min max)) _returnvalue_yaw)) "Undefined" "MultiplyWithRoot" null null)
  (`SceneComponent.SetVisibility` (`self.Ball`) false false))

(fn `ball spawn_Low_Func`
  (params (min :type "Float (double-precision)") (max :type "Float (double-precision)"))
  (bind _asbp_player (cast `/Game/Player/BP_Player` (`GameplayStatics.GetPlayerPawn` 0)))
  (bind (_returnvalue_roll _returnvalue_pitch _returnvalue_yaw) (`KismetMathLibrary.BreakRotator` (`self.K2_GetActorRotation` _asbp_player)))
  (`|SpawnActorFromClass` "/Game/Map/Ball/BP_Ball1.BP_Ball1_C" (`KismetMathLibrary.MakeTransform` (`SceneComponent.K2_GetComponentLocation` (`self.Ball`)) (`KismetMathLibrary.MakeRotator` _returnvalue_roll (+ _returnvalue_pitch (`KismetMathLibrary.RandomFloatInRange` min max)) _returnvalue_yaw)) "Undefined" "MultiplyWithRoot" null null)
  (`SceneComponent.SetVisibility` (`self.Ball`) false false))

(fn `ball spawn_Mid_Func`
  (params (min :type "Float (double-precision)") (max :type "Float (double-precision)"))
  (bind _asbp_player (cast `/Game/Player/BP_Player` (`GameplayStatics.GetPlayerPawn` 0)))
  (bind (_returnvalue_roll _returnvalue_pitch _returnvalue_yaw) (`KismetMathLibrary.BreakRotator` (`self.K2_GetActorRotation` _asbp_player)))
  (`|SpawnActorFromClass` "/Game/Map/Ball/BP_Ball2.BP_Ball2_C" (`KismetMathLibrary.MakeTransform` (`SceneComponent.K2_GetComponentLocation` (`self.Ball`)) (`KismetMathLibrary.MakeRotator` _returnvalue_roll (+ _returnvalue_pitch (`KismetMathLibrary.RandomFloatInRange` min max)) _returnvalue_yaw)) "Undefined" "MultiplyWithRoot" null null)
  (`SceneComponent.SetVisibility` (`self.Ball`) false false))

(fn `UserConstructionScript`)