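; BP_Frame is the target panel of a kick-the-ball strike-out game, with numbered and special cards hit by actors tagged "Ball".
; CardFunc swaps a hit card for a spawned BP_CardGC, disabling its box and hiding its mesh.
; Numbered cards raise the GameInstance's CardCounter; special cards set game over (skull), add kicks (crying) or subtract kicks, floored at zero (smiley).
; Card 9 alone triggers on end overlap, with CardFunc's steps inlined.
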(event `self.BoxA.OnComponentBeginOverlap`
  (params (OverlappedComponent :type "PrimitiveComponent Object Reference") (OtherActor :type "Actor Object Reference") (OtherComp :type "PrimitiveComponent Object Reference") (OtherBodyIndex :type Integer) (bFromSweep :type Boolean) (SweepResult :type "HitResult Structure (by ref)"))
  (if (`self.ActorHasTag` OtherActor "Ball")
    (`self.CardFunc` (`self.BoxA`) (`self.cardA`))
    (bind _asstruc_kout_game_instance (cast `/Game/Map/StrucKOutGameInstance` (`GameplayStatics.GetGameInstance`)))
    (set `/Game/Map/StrucKOutGameInstance.GameOverFlag` true _asstruc_kout_game_instance)
    (`GameplayStatics.PlaySound2D` "/Game/Sound/Boo_QUE.Boo_QUE" 1.0 1.0 0.0 null null)))

(event `self.Box1.OnComponentBeginOverlap`
  (params (OverlappedComponent :type "PrimitiveComponent Object Reference") (OtherActor :type "Actor Object Reference") (OtherComp :type "PrimitiveComponent Object Reference") (OtherBodyIndex :type Integer) (bFromSweep :type Boolean) (SweepResult :type "HitResult Structure (by ref)"))
  (if (`self.ActorHasTag` OtherActor "Ball")
    (`self.CardFunc` (`self.Box1`) (`self.card1`))
    (`self.CardCounter_inc_Func`)
    (`GameplayStatics.PlaySound2D` "/Game/Sound/Yeah_Que.Yeah_Que" 1.0 1.0 0.0 null null)))

(event `self.BoxC.OnComponentBeginOverlap`
  (params (OverlappedComponent :type "PrimitiveComponent Object Reference") (OtherActor :type "Actor Object Reference") (OtherComp :type "PrimitiveComponent Object Reference") (OtherBodyIndex :type Integer) (bFromSweep :type Boolean) (SweepResult :type "HitResult Structure (by ref)"))
  (if (`self.ActorHasTag` OtherActor "Ball")
    (`self.CardFunc` (`self.BoxC`) (`self.cardC`))
    (bind _asstruc_kout_game_instance (cast `/Game/Map/StrucKOutGameInstance` (`GameplayStatics.GetGameInstance`)))
    (bind _returnvalue (- (`/Game/Map/StrucKOutGameInstance.KickCounter` _asstruc_kout_game_instance) 3))
    ; キック数がマイナスになった？？
    (if (< _returnvalue 0)
      (set `/Game/Map/StrucKOutGameInstance.KickCounter` 0 _asstruc_kout_game_instance)
      (else
        (set `/Game/Map/StrucKOutGameInstance.KickCounter` _returnvalue _asstruc_kout_game_instance)))))

(event `self.Box2.OnComponentBeginOverlap`
  (params (OverlappedComponent :type "PrimitiveComponent Object Reference") (OtherActor :type "Actor Object Reference") (OtherComp :type "PrimitiveComponent Object Reference") (OtherBodyIndex :type Integer) (bFromSweep :type Boolean) (SweepResult :type "HitResult Structure (by ref)"))
  (if (`self.ActorHasTag` OtherActor "Ball")
    (`self.CardFunc` (`self.Box2`) (`self.card2`))
    (`self.CardCounter_inc_Func`)
    (`GameplayStatics.PlaySound2D` "/Game/Sound/Yeah_Que.Yeah_Que" 1.0 1.0 0.0 null null)))

(event `self.BoxB.OnComponentBeginOverlap`
  (params (OverlappedComponent :type "PrimitiveComponent Object Reference") (OtherActor :type "Actor Object Reference") (OtherComp :type "PrimitiveComponent Object Reference") (OtherBodyIndex :type Integer) (bFromSweep :type Boolean) (SweepResult :type "HitResult Structure (by ref)"))
  (if (`self.ActorHasTag` OtherActor "Ball")
    (`self.CardFunc` (`self.BoxB`) (`self.cardB`))
    ; キック数を+2するデメリット
    (bind _asstruc_kout_game_instance (cast `/Game/Map/StrucKOutGameInstance` (`GameplayStatics.GetGameInstance`)))
    (set `/Game/Map/StrucKOutGameInstance.KickCounter` (+ (`/Game/Map/StrucKOutGameInstance.KickCounter` _asstruc_kout_game_instance) 2) _asstruc_kout_game_instance)
    (`GameplayStatics.PlaySound2D` "/Game/Sound/Boo_QUE.Boo_QUE" 1.0 1.0 0.0 null null)))

(event `self.Box3.OnComponentBeginOverlap`
  (params (OverlappedComponent :type "PrimitiveComponent Object Reference") (OtherActor :type "Actor Object Reference") (OtherComp :type "PrimitiveComponent Object Reference") (OtherBodyIndex :type Integer) (bFromSweep :type Boolean) (SweepResult :type "HitResult Structure (by ref)"))
  (if (`self.ActorHasTag` OtherActor "Ball")
    (`self.CardFunc` (`self.Box3`) (`self.card3`))
    (`self.CardCounter_inc_Func`)
    (`GameplayStatics.PlaySound2D` "/Game/Sound/Yeah_Que.Yeah_Que" 1.0 1.0 0.0 null null)))

(event `self.Box4.OnComponentBeginOverlap`
  (params (OverlappedComponent :type "PrimitiveComponent Object Reference") (OtherActor :type "Actor Object Reference") (OtherComp :type "PrimitiveComponent Object Reference") (OtherBodyIndex :type Integer) (bFromSweep :type Boolean) (SweepResult :type "HitResult Structure (by ref)"))
  (if (`self.ActorHasTag` OtherActor "Ball")
    (`self.CardFunc` (`self.Box4`) (`self.card4`))
    (`self.CardCounter_inc_Func`)
    (`GameplayStatics.PlaySound2D` "/Game/Sound/Yeah_Que.Yeah_Que" 1.0 1.0 0.0 null null)))

(event `self.Box5.OnComponentBeginOverlap`
  (params (OverlappedComponent :type "PrimitiveComponent Object Reference") (OtherActor :type "Actor Object Reference") (OtherComp :type "PrimitiveComponent Object Reference") (OtherBodyIndex :type Integer) (bFromSweep :type Boolean) (SweepResult :type "HitResult Structure (by ref)"))
  (if (`self.ActorHasTag` OtherActor "Ball")
    (`self.CardFunc` (`self.Box5`) (`self.card5`))
    (`self.CardCounter_inc_Func`)
    (`GameplayStatics.PlaySound2D` "/Game/Sound/Yeah_Que.Yeah_Que" 1.0 1.0 0.0 null null)))

(event `self.Box6.OnComponentBeginOverlap`
  (params (OverlappedComponent :type "PrimitiveComponent Object Reference") (OtherActor :type "Actor Object Reference") (OtherComp :type "PrimitiveComponent Object Reference") (OtherBodyIndex :type Integer) (bFromSweep :type Boolean) (SweepResult :type "HitResult Structure (by ref)"))
  (if (`self.ActorHasTag` OtherActor "Ball")
    (`self.CardFunc` (`self.Box6`) (`self.card6`))
    (`self.CardCounter_inc_Func`)
    (`GameplayStatics.PlaySound2D` "/Game/Sound/Yeah_Que.Yeah_Que" 1.0 1.0 0.0 null null)))

(event `self.Box7.OnComponentBeginOverlap`
  (params (OverlappedComponent :type "PrimitiveComponent Object Reference") (OtherActor :type "Actor Object Reference") (OtherComp :type "PrimitiveComponent Object Reference") (OtherBodyIndex :type Integer) (bFromSweep :type Boolean) (SweepResult :type "HitResult Structure (by ref)"))
  (if (`self.ActorHasTag` OtherActor "Ball")
    (`self.CardFunc` (`self.Box7`) (`self.card7`))
    (`self.CardCounter_inc_Func`)
    (`GameplayStatics.PlaySound2D` "/Game/Sound/Yeah_Que.Yeah_Que" 1.0 1.0 0.0 null null)))

(event `self.Box8.OnComponentBeginOverlap`
  (params (OverlappedComponent :type "PrimitiveComponent Object Reference") (OtherActor :type "Actor Object Reference") (OtherComp :type "PrimitiveComponent Object Reference") (OtherBodyIndex :type Integer) (bFromSweep :type Boolean) (SweepResult :type "HitResult Structure (by ref)"))
  (if (`self.ActorHasTag` OtherActor "Ball")
    (`self.CardFunc` (`self.Box8`) (`self.card8`))
    (`self.CardCounter_inc_Func`)
    (`GameplayStatics.PlaySound2D` "/Game/Sound/Yeah_Que.Yeah_Que" 1.0 1.0 0.0 null null)))

(event `self.Box9.OnComponentEndOverlap`
  (params (OverlappedComponent :type "PrimitiveComponent Object Reference") (OtherActor :type "Actor Object Reference") (OtherComp :type "PrimitiveComponent Object Reference") (OtherBodyIndex :type Integer))
  (bind _box9 (`self.Box9`))
  (bind _card9 (`self.card9`))
  (if (`self.ActorHasTag` OtherActor "Ball")
    (`|SpawnActorFromClass` "/Game/Map/Panel/BP_CardGC.BP_CardGC_C" (`KismetMathLibrary.MakeTransform` (`SceneComponent.K2_GetComponentLocation` _box9) (`SceneComponent.K2_GetComponentRotation` _card9)) "Undefined" "MultiplyWithRoot" null null)
    (`PrimitiveComponent.SetCollisionEnabled` _box9 "NoCollision")
    (`SceneComponent.SetVisibility` _card9 false false)
    (`self.CardCounter_inc_Func`)
    (`GameplayStatics.PlaySound2D` "/Game/Sound/Yeah_Que.Yeah_Que" 1.0 1.0 0.0 null null)))

(fn `CardCounter_inc_Func`
  (bind _asstruc_kout_game_instance (cast `/Game/Map/StrucKOutGameInstance` (`GameplayStatics.GetGameInstance`)))
  (`/Engine/EditorBlueprintResources/StandardMacros.IncrementInt` (`/Game/Map/StrucKOutGameInstance.CardCounter` _asstruc_kout_game_instance)))

(fn `CardFunc`
  (params (box :type "BoxComponent Object Reference") (mesh :type "MeshComponent Object Reference"))
  (`|SpawnActorFromClass` "/Game/Map/Panel/BP_CardGC.BP_CardGC_C" (`KismetMathLibrary.MakeTransform` (`SceneComponent.K2_GetComponentLocation` box) (`SceneComponent.K2_GetComponentRotation` mesh)) "Undefined" "MultiplyWithRoot" null null)
  (`PrimitiveComponent.SetCollisionEnabled` box "NoCollision")
  (`SceneComponent.SetVisibility` mesh false false))

(fn `UserConstructionScript`)