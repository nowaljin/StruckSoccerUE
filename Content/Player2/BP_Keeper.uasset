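; BP_Keeper is the goalkeeper that makes one randomised save attempt when the player kicks.
; Tick polls KickFlag on StrucKOutGameInstance and, through a DoOnce, runs KeeperNoSetFunc once.
; That function uses the BP_Player mesh's yaw sign to randomly choose a right dive, or a centre jump or left dive.
; KeeperNO selects the jump call, and separate jump events play the matching big, small or catch montages.
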(event `self.ReceiveTick`
  (params (DeltaSeconds :type "Float (single-precision)"))
  (bind _asstruc_kout_game_instance (cast `/Game/Map/StrucKOutGameInstance` (`GameplayStatics.GetGameInstance`)))
  (if (`/Game/Map/StrucKOutGameInstance.KickFlag` _asstruc_kout_game_instance)
    (`/Engine/EditorBlueprintResources/StandardMacros.DoOnce` false
      (:`Completed`
        (`self.KeeperNoSetFunc`)
        (switch `int` (`self.KeeperNO`)
          (:`0`
            (`self.C_Jump`))
          (:`1`
            (`self.L_BigJump`))
          (:`2`
            (`self.L_SmallJump`))
          (:`3`
            (`self.R_BigJump`))
          (:`4`
            (`self.R_SmallJump`)))))))

(event `L_BigJump`
  (`self.PlayAnimMontage` "/Game/Player2/animation/KP_DivingSaveL_big_MTG.KP_DivingSaveL_big_MTG"))

(event `R_BigJump`
  (`self.PlayAnimMontage` "/Game/Player2/animation/KP_DirivingSaveR_big_MTG.KP_DirivingSaveR_big_MTG"))

(event `R_SmallJump`
  (`self.PlayAnimMontage` "/Game/Player2/animation/KP_DirivingSaveR_small_MTG.KP_DirivingSaveR_small_MTG"))

(event `L_SmallJump`
  (`self.PlayAnimMontage` "/Game/Player2/animation/KP_DivingSaveL_small_MTG.KP_DivingSaveL_small_MTG"))

(event `C_Jump`
  (`self.PlayAnimMontage` "/Game/Player2/animation/KP_Catch_Jump1_MTG.KP_Catch_Jump1_MTG"))

(fn `KeeperNoSetFunc`
  (bind _returnvalue (`GameplayStatics.GetActorOfClass` "/Game/Player/BP_Player.BP_Player_C"))
  (bind (_returnvalue_roll _returnvalue_pitch _returnvalue_yaw) (`KismetMathLibrary.BreakRotator` (`SceneComponent.K2_GetComponentRotation` (`Character.Mesh` _returnvalue))))
  (if (>= _returnvalue_yaw 0.0)
    (set `self.KeeperNO` (`KismetMathLibrary.RandomIntegerInRange` 3 4))
    (else
      (set `self.KeeperNO` (`KismetMathLibrary.RandomIntegerInRange` 0 2)))))

(fn `UserConstructionScript`)