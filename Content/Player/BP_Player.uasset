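; Player character for what appears to be a soccer game, with camera-relative movement, look controls, a tackle and several kick moves.
; On possession it adds the Enhanced Input mapping context, and input actions drive movement, rotation and montage playback.
; Each shot input also sets KickST to identify the kick type: inside, main or running.
; FootCollisionON and FootCollisionOFF events toggle the FootBox collision, with no caller in this graph.
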(event `self.ReceiveTick`
  (params (DeltaSeconds :type "Float (single-precision)")))

(event `self.ReceivePossessed`
  (params (NewController :type "Controller Object Reference"))
  ; キーの初期化
  (bind `_asプレイヤーコントローラー` (cast `PlayerController` NewController))
  (message `EnhancedInputSubsystemInterface.AddMappingContext` (pcsubsystem `EnhancedInputLocalPlayerSubsystem` `_asプレイヤーコントローラー`) "/Game/Player/input/IA_Player.IA_Player" 0 (struct)))

(event `EnhancedInput|/Game/Player/input/IA_attack`
  (params (ActionValue :type Boolean) (ElapsedSeconds :type "Float (double-precision)") (TriggeredSeconds :type "Float (double-precision)") (InputAction :type "InputAction Object Reference" :default "/Game/Player/input/IA_attack.IA_attack"))
  ; 視点切り替えとジャンプ
  (:`Triggered`
    (`self.PlayAnimMontage` "/Game/Player/animations/PTackle_MTG.PTackle_MTG")))

(event `EnhancedInput|/Game/Player/input/IA_MouseL`
  (params (ActionValue :type Boolean) (ElapsedSeconds :type "Float (double-precision)") (TriggeredSeconds :type "Float (double-precision)") (InputAction :type "InputAction Object Reference" :default "/Game/Player/input/IA_MouseL.IA_MouseL"))
  (:`Triggered`
    (`self.PlayAnimMontage` "/Game/Player/animations/P1shoot_main_MTG.P1shoot_main_MTG")
    (set `self.kickST` 2)))

(event `EnhancedInput|/Game/Player/input/IA_Turn`
  (params (ActionValue :type "Float (double-precision)") (ElapsedSeconds :type "Float (double-precision)") (TriggeredSeconds :type "Float (double-precision)") (InputAction :type "InputAction Object Reference" :default "/Game/Player/input/IA_Turn.IA_Turn"))
  ; 視点切り替えとジャンプ
  (:`Triggered`
    (`self.AddControllerYawInput` ActionValue)))

(event `EnhancedInput|/Game/Player/input/IA_MouseR`
  (params (ActionValue :type Boolean) (ElapsedSeconds :type "Float (double-precision)") (TriggeredSeconds :type "Float (double-precision)") (InputAction :type "InputAction Object Reference" :default "/Game/Player/input/IA_MouseR.IA_MouseR"))
  (:`Triggered`
    (`self.PlayAnimMontage` "/Game/Player/animations/P2Shoot_run_MTG.P2Shoot_run_MTG")
    (set `self.kickST` 3)))

(event `EnhancedInput|/Game/Player/input/IA_LookUp`
  (params (ActionValue :type "Float (double-precision)") (ElapsedSeconds :type "Float (double-precision)") (TriggeredSeconds :type "Float (double-precision)") (InputAction :type "InputAction Object Reference" :default "/Game/Player/input/IA_LookUp.IA_LookUp"))
  ; 視点切り替えとジャンプ
  (:`Triggered`
    (`self.AddControllerPitchInput` ActionValue)))

(event `EnhancedInput|/Game/Player/input/IA_inside1`
  (params (ActionValue :type Boolean) (ElapsedSeconds :type "Float (double-precision)") (TriggeredSeconds :type "Float (double-precision)") (InputAction :type "InputAction Object Reference" :default "/Game/Player/input/IA_inside1.IA_inside1"))
  (:`Triggered`
    (`self.PlayAnimMontage` "/Game/Player/animations/P1shoot_inside1_MTG.P1shoot_inside1_MTG")
    (set `self.kickST` 1 :!label _label)))

(event `EnhancedInput|/Game/Player/input/IA_WS`
  (params (ActionValue :type "Float (double-precision)") (ElapsedSeconds :type "Float (double-precision)") (TriggeredSeconds :type "Float (double-precision)") (InputAction :type "InputAction Object Reference" :default "/Game/Player/input/IA_WS.IA_WS"))
  (bind (_returnvalue_roll _returnvalue_pitch _returnvalue_yaw) (`KismetMathLibrary.BreakRotator` (`self.GetControlRotation`)))
  ; 移動
  (:`Triggered`
    (`self.AddMovementInput` (`KismetMathLibrary.GetForwardVector` (`KismetMathLibrary.MakeRotator` 0.0 0.0 _returnvalue_yaw)) ActionValue)))

(event `EnhancedInput|/Game/Player/input/IA_inside2`
  (params (ActionValue :type Boolean) (ElapsedSeconds :type "Float (double-precision)") (TriggeredSeconds :type "Float (double-precision)") (InputAction :type "InputAction Object Reference" :default "/Game/Player/input/IA_inside2.IA_inside2"))
  (:`Triggered`
    (`self.PlayAnimMontage` "/Game/Player/animations/P1shoot_inside2_MTG.P1shoot_inside2_MTG")
    (goto _label)))

(event `EnhancedInput|/Game/Player/input/IA_AD`
  (params (ActionValue :type "Float (double-precision)") (ElapsedSeconds :type "Float (double-precision)") (TriggeredSeconds :type "Float (double-precision)") (InputAction :type "InputAction Object Reference" :default "/Game/Player/input/IA_AD.IA_AD"))
  (bind (_returnvalue_roll _returnvalue_pitch _returnvalue_yaw) (`KismetMathLibrary.BreakRotator` (`self.GetControlRotation`)))
  ; 移動
  (:`Triggered`
    (`self.AddMovementInput` (`KismetMathLibrary.GetRightVector` (`KismetMathLibrary.MakeRotator` 0.0 0.0 _returnvalue_yaw)) ActionValue)))

(event `FootCollisionON`
  ; FootコリジョンのＯＮ／ＯＦＦ
  (`PrimitiveComponent.SetCollisionEnabled` (`self.FootBox`) "QueryAndPhysics"))

(event `FootCollisionOFF`
  ; FootコリジョンのＯＮ／ＯＦＦ
  (`PrimitiveComponent.SetCollisionEnabled` (`self.FootBox`) "NoCollision"))

(fn `UserConstructionScript`)